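; BP_PointCloud is an actor that stores and renders lidar points as instanced sphere meshes.
; Its construction script creates a shadowless, collision-free instanced static mesh component with one custom data float.
; AddPoint places an instance aligned to the given normal and writes the enemy flag into that float.
; Once MaxPoints is reached, a wrapping index overwrites existing instances like a ring buffer, capping the cloud's size.
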(event EventBeginPlay)

(event Collision|EventActorBeginOverlap
  (params (OtherActor :type Actor%20Object%20Reference)))

(event EventTick
  (params (DeltaSeconds :type Float%20%28single-precision%29)))

(fn ConstructionScript
  (bind _returnvalue (AddComponent|AddInstancedStaticMeshComponent false))
  (Variables|Default|SetISM _returnvalue)
  (Components|StaticMesh|SetStaticMesh _returnvalue "/Game/Lidar/SM_PointSphere.SM_PointSphere")
  (Class|InstancedStaticMeshComponent|SetNumCustomDataFloats _returnvalue 1)
  (Rendering|SetCastShadow _returnvalue false)
  (Collision|SetCollisionEnabled _returnvalue "NoCollision"))

(fn AddPoint
  (params (Location :type Vector) (IsEnemy :type Float%20%28double-precision%29) (Normal :type Vector))
  (bind _returnvalue (Math|Rotator|MakeRotfromZ Normal))
  (bind _returnvalue_2 (* Normal ""))
  (bind _pointscale (Variables|Default|GetPointScale))
  (bind _ism (Variables|Default|GetISM))
  (bind _maxpoints (Variables|Default|GetMaxPoints))
  (bind _returnvalue_3 (Math|Vector|MakeVector _pointscale _pointscale _pointscale))
  (bind _returnvalue_4 (+ Location _returnvalue_2))
  (bind _returnvalue_5 (Math|Transform|MakeTransform _returnvalue_4 _returnvalue _returnvalue_3))
  (if (< (Components|InstancedStaticMesh|GetInstanceCount _ism) _maxpoints)
    (bind _returnvalue_6 (Components|InstancedStaticMesh|AddInstance _ism _returnvalue_5 true))
    (Components|InstancedStaticMesh|SetCustomDataValue _ism _returnvalue_6 0 IsEnemy true)
    (else
      (Components|InstancedStaticMesh|UpdateInstanceTransform _ism (Variables|Default|GetNextIndex) _returnvalue_5 true true false)
      (Components|InstancedStaticMesh|SetCustomDataValue _ism (Variables|Default|GetNextIndex) 0 IsEnemy true)
      (Variables|Default|SetNextIndex (+ (Variables|Default|GetNextIndex) 1))
      (if (>= (Variables|Default|GetNextIndex) _maxpoints)
        (Variables|Default|SetNextIndex 0)))))

(fn BuildCloud0)